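; Game mode that sets up input focus and render settings at startup and tracks whether the player is using a controller.
; BeginPlay sets Game and UI input mode focused on the first top-level BP_VillageUI widget, then applies screen percentage and scalability through console commands.
; Tick polls the controller-input flag against its cached value and calls the ChangeInputFeedback dispatcher only when it changes.
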(event EventBeginPlay
  (bind _foundwidgets (Widget|GetAllWidgetsOfClass "/Game/Blueprint/VillageSystem/Widget/BP_VillageUI.BP_VillageUI_C" true))
  (Input|SetInputModeGameandUI (Game|GetPlayerController 0) (Utilities|Array|Get(acopy) _foundwidgets) "DoNotLock" true false)
  (Development|ExecuteConsoleCommand " r.ScreenPercentage 170" 0)
  (Development|ExecuteConsoleCommand "Scalability 1" 0))

(event EventTick
  (params (DeltaSeconds :type Float%20%28single-precision%29))
  (if (not (== (Variables|Default|GetIsControllerInput) (Variables|Default|GetCurrentControllerInput)))
    (Variables|Default|SetCurrentControllerInput (Variables|Default|GetIsControllerInput))
    (Default|CallChangeInputFeedback)))

(fn ConstructionScript)