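; Player character Blueprint that drives two trail effects from movement speed every Tick.
; The Velocity Normalize helper's scalar scales Trail1's minimum and maximum size and Trail2's upward Z velocity, each above a base value.
; That helper contains a current-speed over max-speed calculation, though it appears unconnected to any output.
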(event EventTick
  (params (DeltaSeconds :type Float%20%28single-precision%29))
  (bind _returnvalue (Utilities|VelocityNormalize))
  (bind _trail_1 (Variables|Default|GetTrail%201))
  (Niagara|SetNiagaraVariable(Float) _trail_1 "MaxSize" (+ (* _returnvalue 4e+02) 4e+02))
  (Niagara|SetNiagaraVariable(Float) _trail_1 "MinSize" (+ (* _returnvalue 1.5e+02) 1.5e+02))
  (Niagara|SetNiagaraVariable(Vector3) (Variables|Default|GetTrail%202) "Velocity" (Math|Vector|MakeVector 0.0 0.0 (+ (* _returnvalue 4e+02) 2e+02))))

(fn ConstructionScript)