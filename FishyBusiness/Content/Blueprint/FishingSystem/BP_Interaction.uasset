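; BP_Interaction is an interaction prompt actor in the fishing system, with controller and keyboard variants.
; The GameMode's input-feedback event switches which variant is visible, based on IsControllerInput.
; Both share a dynamic material whose opacity is timeline-driven, with the same curve offsetting the actor's height from its spawn point.
; The intro animation plays on BeginPlay, while DestroyCall plays the outro and then destroys the actor.
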(event Custom|SwitchInteractionUI
  (bind _asgm_game_mode (Utilities|Casting|CastToGM_GameMode (Game|GetGameMode)))
  (if (Variables|/Game/GM_GameMode.GM_GameMode_C|GetIsControllerInput _asgm_game_mode)
    (Development|SetHiddeninGame (Variables|Default|GetInteractionC) false false)
    (Development|SetHiddeninGame (Variables|Default|GetInteractionKB) true false)
    (else
      (Development|SetHiddeninGame (Variables|Default|GetInteractionC) true false)
      (Development|SetHiddeninGame (Variables|Default|GetInteractionKB) false false))))

(event Custom|DestroyCall
  (bind _transparency (Timeline|FinalAnimation Play)
    (:Update
      (Rendering|Material|SetScalarParameterValue (Variables|Default|GetMaterial%20Instance) "Opacity" _transparency :!class /Script/Engine.MaterialInstanceDynamic)
      (Transformation|SetActorLocation (+ (Variables|Default|GetInitialLocation) (Math|Vector|MakeVector 0.0 0.0 (* _transparency 4e+02))) false false))
    (:Finished
      (Actor|DestroyActor))))

(event EventBeginPlay
  (bind _returnvalue (Rendering|Material|CreateDynamicMaterialInstance "/Game/Materials/MaterialIstances/MI_TB_Interaction.MI_TB_Interaction" "None" "None" :!class /Script/Engine.KismetMaterialLibrary))
  (Variables|Default|SetMaterial%20Instance _returnvalue)
  (Rendering|Material|SetMaterial (Variables|Default|GetInteractionC) 0 _returnvalue)
  (Rendering|Material|SetMaterial (Variables|Default|GetInteractionKB) 0 _returnvalue)
  (Utilities|FlowControl|Sequence
    (:then_0
      (bind _asgm_game_mode (Utilities|Casting|CastToGM_GameMode (Game|GetGameMode)))
      (EventDispatchers|BindEventtoChangeInputFeedback _asgm_game_mode (delegate Custom|SwitchInteractionUI))
      (bind _asgm_game_mode_2 (Utilities|Casting|CastToGM_GameMode (Game|GetGameMode)))
      (if (Variables|/Game/GM_GameMode.GM_GameMode_C|GetIsControllerInput _asgm_game_mode_2)
        (Development|SetHiddeninGame (Variables|Default|GetInteractionC) false false)
        (Development|SetHiddeninGame (Variables|Default|GetInteractionKB) true false)
        (else
          (Development|SetHiddeninGame (Variables|Default|GetInteractionC) true false)
          (Development|SetHiddeninGame (Variables|Default|GetInteractionKB) false false))))
    (:then_1
      (Variables|Default|SetInitialLocation (Transformation|GetActorLocation))
      (bind _transparency (Timeline|InitialAnimation Play)
        (:Update
          (Rendering|Material|SetScalarParameterValue (Variables|Default|GetMaterial%20Instance) "Opacity" _transparency :!class /Script/Engine.MaterialInstanceDynamic)
          (Transformation|SetActorLocation (+ (Variables|Default|GetInitialLocation) (Math|Vector|MakeVector 0.0 0.0 (* _transparency 4e+02))) false false))))))

(fn ConstructionScript)