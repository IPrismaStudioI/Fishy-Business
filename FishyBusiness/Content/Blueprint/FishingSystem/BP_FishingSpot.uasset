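; BP_FishingSpot is a fishing-spot actor that shows an interaction prompt while the player character is near it.
; Its sphere trigger creates a WBP_Interaction widget on overlap, stores it in the character's InteractUI and adds it to the viewport, then removes it on exit.
; A separate helper, UpdateGMControllerStatus, sets the game mode's IsControllerInput flag according to whether a given key is a gamepad key.
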(event OnComponentBeginOverlap(xSphereTrigger)
  (params (OverlappedComponent :type Primitive%20Component%20Object%20Reference) (OtherActor :type Actor%20Object%20Reference) (OtherComp :type Primitive%20Component%20Object%20Reference) (OtherBodyIndex :type Integer) (bFromSweep :type Boolean) (SweepResult :type Hit%20Result%20Structure%20%28by%20ref%29))
  (bind _asbp_player_character (Utilities|Casting|CastToBP_PlayerCharacter OtherActor))
  (bind _returnvalue (UserInterface|CreateWidget "/Game/Blueprint/FishingSystem/WBP_Interaction.WBP_Interaction_C"))
  (bind _output_get (Variables|/Game/Blueprint/PlayerSystem/BP_PlayerCharacter.BP_PlayerCharacter_C|SetInteractUI _asbp_player_character _returnvalue))
  (UserInterface|Viewport|AddtoViewport _output_get 0))

(event OnComponentEndOverlap(xSphereTrigger)
  (params (OverlappedComponent :type Primitive%20Component%20Object%20Reference) (OtherActor :type Actor%20Object%20Reference) (OtherComp :type Primitive%20Component%20Object%20Reference) (OtherBodyIndex :type Integer))
  (bind _asbp_player_character (Utilities|Casting|CastToBP_PlayerCharacter OtherActor))
  (Widget|RemovefromParent (Variables|/Game/Blueprint/PlayerSystem/BP_PlayerCharacter.BP_PlayerCharacter_C|GetInteractUI _asbp_player_character)))

(fn ConstructionScript)

(fn UpdateGMControllerStatus
  (params (KeyInput :type Key%20Structure :default "None"))
  (bind _asgm_game_mode (Utilities|Casting|CastToGM_GameMode (Game|GetGameMode)))
  (if (Class|KismetInputLibrary|KeyIsGamepadKey KeyInput)
    (Variables|/Game/GM_GameMode.GM_GameMode_C|SetIsControllerInput _asgm_game_mode true)
    (else
      (Variables|/Game/GM_GameMode.GM_GameMode_C|SetIsControllerInput _asgm_game_mode false))))