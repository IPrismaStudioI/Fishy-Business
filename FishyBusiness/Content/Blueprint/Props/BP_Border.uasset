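; BP_Border is a prop Blueprint that enlarges itself once the tutorial quest is completed.
; On Tick, a DoOnce checks the FishyBusiness game mode's completed quest list for TutorialID.
; When the ID is found, the root scales up horizontally to triple size and the check stays closed; otherwise it resets the DoOnce to poll again next frame.
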(event EventTick
  (params (DeltaSeconds :type Float%20%28single-precision%29))
  (Utilities|FlowControl|DoOnce false :!label _label
    (:Completed
      (bind _asfishy_business_game_mode_base (Utilities|Casting|CastToFishyBusinessGameModeBase (Game|GetGameMode)))
      (if (!= (Utilities|Array|FindItem (Variables|/Script/FishyBusiness.QuestUnlockStorageManager|Get_sCompletedQuestList (Variables|/Script/FishyBusiness.FishyBusinessGameModeBase|GetxQuestUnlockStorageManager _asfishy_business_game_mode_base)) (Variables|Default|GetTutorialID)) -1)
        (Transformation|SetWorldScale3D (Variables|Default|GetDefaultSceneRoot) "3.000000,3.000000,1.000000")
        (else
          (goto _label Reset))))))

(fn ConstructionScript)