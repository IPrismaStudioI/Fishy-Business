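; Tutorial fishing generator that shows its fishing spots only while the tutorial quest identified by TutorialID is relevant.
; On BeginPlay it hides each spot's fish meshes and disables its trigger collision.
; Tick polls through self-resetting DoOnce gates, revealing the spots once the quest is in the player's quest log.
; When the game mode's completed-quest list contains that ID, it destroys the spots and itself.
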(event EventTick
  (params (DeltaSeconds :type Float%20%28single-precision%29))
  (Utilities|FlowControl|Sequence
    (:then_0
      (Utilities|FlowControl|DoOnce false :!label _label
        (:Completed
          (bind _asbp_player_character (Utilities|Casting|CastToBP_PlayerCharacter (Pawn|GetControlledPawn (Game|GetPlayerController 0))))
          (if (.ReturnValue (Utilities|Map|Find (Variables|/Script/FishyBusiness.AC_QuestLog|GetxQuests (Variables|/Script/FishyBusiness.PlayerCharacter|GetxQuestLog _asbp_player_character)) (Variables|Default|GetTutorial%20ID)))
            (CallFunction|ChangeHiddenFIshingSpot false "QueryOnly")
            (else
              (goto _label Reset))))))
    (:then_1
      (Utilities|FlowControl|DoOnce false :!label _label_2
        (:Completed
          (bind _asfishy_business_game_mode_base (Utilities|Casting|CastToFishyBusinessGameModeBase (Game|GetGameMode)))
          (if (!= (Utilities|Array|FindItem (Variables|/Script/FishyBusiness.QuestUnlockStorageManager|Get_sCompletedQuestList (Variables|/Script/FishyBusiness.FishyBusinessGameModeBase|GetxQuestUnlockStorageManager _asfishy_business_game_mode_base)) (Variables|Default|GetTutorial%20ID)) -1)
            (CallFunction|DestroyFIshingGenerator)
            (else
              (goto _label_2 Reset))))))))

(event EventBeginPlay
  (CallFunction|ChangeHiddenFIshingSpot true "NoCollision"))

(fn ConstructionScript)

(fn DestroyFIshingGenerator
  (for _array_element (Variables|Default|GetxFishingSpots)
    (Actor|DestroyActor _array_element))
  (Actor|DestroyActor))

(fn ChangeHiddenFIshingSpot
  (params (IsHidden :type Boolean) (Type :type ECollisionEnabled%20Enum :default "NoCollision"))
  (for _array_element (Variables|Default|GetxFishingSpots)
    (Collision|SetCollisionEnabled (Variables|/Script/FishyBusiness.FishingSpot|GetxSphereTrigger _array_element) Type)
    (bind _asbp_fishing_spot (Utilities|Casting|CastToBP_FishingSpot _array_element))
    (for _array_element_2 (Utilities|Array|MakeArray (Variables|/Game/Blueprint/FishingSystem/BP_FishingSpot.BP_FishingSpot_C|GetFish _asbp_fishing_spot) (Variables|/Game/Blueprint/FishingSystem/BP_FishingSpot.BP_FishingSpot_C|GetFish1 _asbp_fishing_spot) (Variables|/Game/Blueprint/FishingSystem/BP_FishingSpot.BP_FishingSpot_C|GetFish2 _asbp_fishing_spot))
      (Development|SetHiddeninGame _array_element_2 IsHidden false))))