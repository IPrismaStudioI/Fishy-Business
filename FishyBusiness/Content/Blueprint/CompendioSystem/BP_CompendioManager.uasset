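; Compendium manager that handles input for opening, closing and paging the in-game compendium.
; The open input branches on the player's overlay state to play open or close sounds and flip the open flag, while closing also fires the CompendioIsClosing dispatcher.
; Closing and page-turn inputs dismiss polaroid overlays.
; Open and page inputs also tell the game mode whether keyboard or controller is in use.
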(event Custom|ChangeCompendioStatus
  (bind _asbp_player_character (Utilities|Casting|CastToBP_PlayerCharacter (Pawn|GetControlledPawn (Game|GetPlayerController 0))))
  (if (Variables|/Game/Blueprint/PlayerSystem/BP_PlayerCharacter.BP_PlayerCharacter_C|GetIsOverlayOpen _asbp_player_character)
    (if (Variables|Default|GetIs%20CompendioOpen)
      (Class|FMODBlueprintStatics|PlayEvent2D "/Game/FMOD/Events/FOLDER_CompendiumAndMap/SFX_CompendiumClose.SFX_CompendiumClose")
      (Default|CallCompendioIsClosing)
      (bind _foundwidgets (Widget|GetAllWidgetsOfClass "/Game/Blueprint/CompendioSystem/Page/Base/WBP_PolaroidOverlay.WBP_PolaroidOverlay_C" true))
      (for _array_element _foundwidgets
        (Default|ClosePolaroid _array_element))
      (Variables|Default|SetIs%20CompendioOpen (not (Variables|Default|GetIs%20CompendioOpen)) :!label _label))
    (else
      (Class|FMODBlueprintStatics|PlayEvent2D "/Game/FMOD/Events/FOLDER_CompendiumAndMap/SFX_CompendiumOpen.SFX_CompendiumOpen")
      (goto _label))))

(event Input|ActionEvents|InputActionOpenCompendio
  (params (Key :type Key%20Structure :default "None"))
  (:Pressed
    (CallFunction|UpdateGMControllerStatus Key)
    (bind _asbp_player_character (Utilities|Casting|CastToBP_PlayerCharacter (Pawn|GetControlledPawn (Game|GetPlayerController 0))))
    (if (Variables|/Game/Blueprint/PlayerSystem/BP_PlayerCharacter.BP_PlayerCharacter_C|GetIsOverlayOpen _asbp_player_character)
      (if (Variables|Default|GetIs%20CompendioOpen)
        (Class|FMODBlueprintStatics|PlayEvent2D "/Game/FMOD/Events/FOLDER_CompendiumAndMap/SFX_CompendiumClose.SFX_CompendiumClose")
        (Default|CallCompendioIsClosing)
        (bind _foundwidgets (Widget|GetAllWidgetsOfClass "/Game/Blueprint/CompendioSystem/Page/Base/WBP_PolaroidOverlay.WBP_PolaroidOverlay_C" true))
        (for _array_element _foundwidgets
          (Default|ClosePolaroid _array_element))
        (Variables|Default|SetIs%20CompendioOpen (not (Variables|Default|GetIs%20CompendioOpen)) :!label _label))
      (else
        (Class|FMODBlueprintStatics|PlayEvent2D "/Game/FMOD/Events/FOLDER_CompendiumAndMap/SFX_CompendiumOpen.SFX_CompendiumOpen")
        (goto _label)))))

(event Input|ActionEvents|InputActionNextCompendioPage
  (params (Key :type Key%20Structure :default "None"))
  (:Pressed
    (CallFunction|UpdateGMControllerStatus Key)
    (bind _foundwidgets (Widget|GetAllWidgetsOfClass "/Game/Blueprint/CompendioSystem/Page/Base/WBP_PolaroidOverlay.WBP_PolaroidOverlay_C" true))
    (for _array_element _foundwidgets
      (Default|ClosePolaroid _array_element))))

(event Input|ActionEvents|InputActionCloseCompendio
  (params (Key :type Key%20Structure :default "None"))
  (:Pressed
    (if (Variables|Default|GetIs%20CompendioOpen)
      (Class|FMODBlueprintStatics|PlayEvent2D "/Game/FMOD/Events/FOLDER_CompendiumAndMap/SFX_CompendiumClose.SFX_CompendiumClose")
      (Default|CallCompendioIsClosing)
      (bind _foundwidgets (Widget|GetAllWidgetsOfClass "/Game/Blueprint/CompendioSystem/Page/Base/WBP_PolaroidOverlay.WBP_PolaroidOverlay_C" true))
      (for _array_element _foundwidgets
        (Default|ClosePolaroid _array_element))
      (Variables|Default|SetIs%20CompendioOpen (not (Variables|Default|GetIs%20CompendioOpen))))))

(event Input|ActionEvents|InputActionPrevCompendioPage
  (params (Key :type Key%20Structure :default "None"))
  (:Pressed
    (CallFunction|UpdateGMControllerStatus Key)
    (bind _foundwidgets (Widget|GetAllWidgetsOfClass "/Game/Blueprint/CompendioSystem/Page/Base/WBP_PolaroidOverlay.WBP_PolaroidOverlay_C" true))
    (for _array_element _foundwidgets
      (Default|ClosePolaroid _array_element))))

(fn ConstructionScript)

(fn UpdateGMControllerStatus
  (params (KeyInput :type Key%20Structure :default "None"))
  (bind _asgm_game_mode (Utilities|Casting|CastToGM_GameMode (Game|GetGameMode)))
  (if (Class|KismetInputLibrary|KeyIsKeyboardKey KeyInput)
    (Variables|/Game/GM_GameMode.GM_GameMode_C|SetIsControllerInput _asgm_game_mode false)
    (else
      (Variables|/Game/GM_GameMode.GM_GameMode_C|SetIsControllerInput _asgm_game_mode true))))