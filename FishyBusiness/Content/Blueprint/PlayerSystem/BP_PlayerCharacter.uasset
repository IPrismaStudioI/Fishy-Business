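; Player boat character that owns the HUD and pause menu, and drives movement trail effects and sound.
; Tick scales two trail effects by normalized speed, starts or stops the FMOD boat sound, and watches game mode overlay visibility through DoOnce gates.
; Overlay and interaction events toggle the HUD and interaction actor, with hiding also recording gamepad input on the game mode.
; P toggles the pause menu outside the main menu when no overlay is visible.
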(event Custom|Show%20Interaction%20Overlay
  (CallFunction|CloseMainOverlay)
  (bind _interactionbp (Variables|Default|GetInteractionBP)
    (:then
      (Rendering|SetActorHiddenInGame _interactionbp false))
    (:else)))

(event Custom|Hide%20Interaction%20UI
  (params (Input :type Key%20Structure :default "None"))
  (bind _interactionbp (Variables|Default|GetInteractionBP)
    (:then
      (CallFunction|UpdateGMControllerStatus Input)
      (Rendering|SetActorHiddenInGame _interactionbp true)
      (CallFunction|OpenMainOverlay))
    (:else)))

(event Custom|OpenMainOverlay
  (Default|CloseHUD (Variables|Default|GetHUD))
  (Variables|Default|SetIsOverlayOpen true))

(event Custom|CloseMainOverlay
  (Default|OpenHUD (Variables|Default|GetHUD))
  (Variables|Default|SetIsOverlayOpen false))

(event EventBeginPlay
  (bind _returnvalue (UserInterface|CreateWidget "/Game/Blueprint/Widgets/HUD/WBP_HUD.WBP_HUD_C"))
  (bind _output_get (Variables|Default|SetHUD _returnvalue))
  (UserInterface|Viewport|AddtoViewport _output_get 0)
  (Utilities|FlowControl|Sequence
    (:then_0
      (bind _returnvalue_2 (Game|GetCurrentLevelName true))
      (if (Utilities|Enum|Equal(Enum) _returnvalue_2 "scn_MainMenu")
        (Widget|SetVisibility _output_get "Collapsed")))
    (:then_1
      (bind _returnvalue_3 (UserInterface|CreateWidget "/Game/Blueprint/Widgets/Misc/WBP_PauseMenu.WBP_PauseMenu_C"))
      (bind _output_get_2 (Variables|Default|SetPause%20Menu _returnvalue_3))
      (UserInterface|Viewport|AddtoViewport _output_get_2 0)
      (Widget|SetVisibility _output_get_2 "Collapsed"))))

(event EventTick
  (params (DeltaSeconds :type Float%20%28single-precision%29))
  (bind _returnvalue (Utilities|VelocityNormalize))
  (bind _trail_1 (Variables|Default|GetTrail%201))
  (bind _trail_2 (Variables|Default|GetTrail%202))
  (Niagara|SetNiagaraVariable(Float) _trail_1 "MaxSize" (+ (* _returnvalue 4e+02) 4e+02))
  (Niagara|SetNiagaraVariable(Float) _trail_1 "MinSize" (+ (* _returnvalue 1.5e+02) 1.5e+02))
  (Niagara|SetNiagaraVariable(Vector3) _trail_2 "Velocity" (Math|Vector|MakeVector 0.0 0.0 (+ (* _returnvalue 4e+02) 2e+02)))
  (Niagara|SetNiagaraVariable(Float) _trail_2 "SpawnCount" (* _returnvalue 5e+01))
  (Utilities|FlowControl|Sequence
    (:then_0
      (if (Variables|Default|GetbIsMoving)
        (Utilities|FlowControl|DoOnce false :!label _label
          (:Completed
            (bind _returnvalue_2 (Class|FMODBlueprintStatics|PlayEvent2D "/Game/FMOD/Events/FOLDER_Boat/SFX_BoatMovement.SFX_BoatMovement"))))
        (else
          (Class|FMODBlueprintStatics|EventInstanceStop _returnvalue_2 false)
          (goto _label Reset))))
    (:then_1
      (bind _asfishy_business_game_mode_base (Utilities|Casting|CastToFishyBusinessGameModeBase (Game|GetGameMode)))
      (if (Class|FishyBusinessGameModeBase|GetIsMainOverlayVisible _asfishy_business_game_mode_base)
        (Utilities|FlowControl|DoOnce false :!label _label_2
          (:Completed
            (CallFunction|OpenMainOverlay)
            (goto _label_3 Reset)))
        (else
          (Utilities|FlowControl|DoOnce false :!label _label_3
            (:Completed
              (CallFunction|CloseMainOverlay)
              (goto _label_2 Reset))))))))

(event Input|KeyboardEvents|P
  (params (Key :type Key%20Structure :default "None"))
  (:Pressed
    (bind _returnvalue (Game|GetCurrentLevelName true))
    (if (not (Utilities|Enum|Equal(Enum) _returnvalue "scn_MainMenu"))
      (bind _asfishy_business_game_mode_base (Utilities|Casting|CastToFishyBusinessGameModeBase (Game|GetGameMode)))
      (if (not (Class|FishyBusinessGameModeBase|GetIsMainOverlayVisible _asfishy_business_game_mode_base))
        (if (Variables|Default|GetIs%20pause%20menu%20open)
          (Widget|SetVisibility (Variables|Default|GetPause%20Menu) "Collapsed")
          (Variables|Default|SetIs%20pause%20menu%20open false)
          (else
            (Widget|SetVisibility (Variables|Default|GetPause%20Menu) "Visible")
            (Variables|Default|SetIs%20pause%20menu%20open true)))))))

(fn ConstructionScript)

(fn UpdateGMControllerStatus
  (params (KeyInput :type Key%20Structure :default "None"))
  (bind _asgm_game_mode (Utilities|Casting|CastToGM_GameMode (Game|GetGameMode)))
  (if (Class|KismetInputLibrary|KeyIsGamepadKey KeyInput)
    (Variables|/Game/GM_GameMode.GM_GameMode_C|SetIsControllerInput _asgm_game_mode true)
    (else
      (Variables|/Game/GM_GameMode.GM_GameMode_C|SetIsControllerInput _asgm_game_mode false))))