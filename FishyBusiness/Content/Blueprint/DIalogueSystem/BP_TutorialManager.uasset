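; BP_TutorialManager is an actor that runs the intro dialogue sequence, then hands over to a reward overlay.
; BeginPlay waits briefly, shows WBP_DialogueIntro and resets a DoOnce.
; Tick polls the dialogue canvas, reached through the game mode's dialogue elaborator, and fires that DoOnce when it is collapsed.
; This removes the intro, adds WBP_RewardOverlay to the viewport and destroys the manager.
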(event EventTick
  (params (DeltaSeconds :type Float%20%28single-precision%29))
  (bind _asfishy_business_game_mode_base (Utilities|Casting|CastToFishyBusinessGameModeBase (Game|GetGameMode)))
  (bind _aswbp_dialogue_ui (Utilities|Casting|CastToWBP_DialogueUI (Variables|/Script/FishyBusiness.DialogueElaborator|GetdialogueUIWidget (Variables|/Script/FishyBusiness.FishyBusinessGameModeBase|GetxDialogueElaborator _asfishy_business_game_mode_base))))
  (if (Utilities|Enum|Equal(Enum) (Variables|/Script/UMG.Widget|GetVisibility (Variables|/Script/FishyBusiness.DialogueUI|Get_xCanvasDialogue _aswbp_dialogue_ui)) "Collapsed")
    (Utilities|FlowControl|DoOnce true
      (:Completed
        (Widget|RemovefromParent (stale EventBeginPlay _returnvalue))
        (bind _returnvalue (UserInterface|CreateWidget "/Game/Blueprint/Widgets/Misc/WBP_RewardOverlay.WBP_RewardOverlay_C"))
        (UserInterface|Viewport|AddtoViewport _returnvalue 0)
        (Actor|DestroyActor)))))

(event EventBeginPlay
  (Utilities|FlowControl|Delay 0.2)
  (bind _returnvalue (UserInterface|CreateWidget "/Game/Blueprint/DIalogueSystem/WBP_DialogueIntro.WBP_DialogueIntro_C"))
  (UserInterface|Viewport|AddtoViewport _returnvalue 0)
  (Utilities|FlowControl|DoOnce true) ; enters at Reset
)

(fn ConstructionScript)