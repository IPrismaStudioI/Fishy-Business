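; BP_CompendioManager toggles an in-game compendium screen with open and close sounds.
; On BeginPlay it creates a hidden WBP_MainCompendio widget in the viewport and enables input for player 0.
; The C key and the Open/CloseCompendium event share one toggle of IsCompendium.
; Opening shows the widget and adds its first two pages, while closing hides it and calls RemovePage.
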(event Custom|Open/Close%20Compendium
  (bind _compendio (Variables|Default|GetCompendio))
  (bind _compendio_2 (Variables|Default|GetCompendio))
  (bind _output_get (Variables|Default|SetIs%20Compendium (not (Variables|Default|GetIs%20Compendium))))
  (if _output_get
    (Widget|SetVisibility _compendio "Visible")
    (Default|AddPage _compendio)
    (Default|AddPage _compendio 1)
    (Audio|PlaySound2D "/Game/Sound/SFX/SFX_CompendiumOpen.SFX_CompendiumOpen" 1.0 1.0 0.0 0 0)
    (else
      (Widget|SetVisibility _compendio_2 "Hidden")
      (Default|RemovePage _compendio_2)
      (Audio|PlaySound2D "/Game/Sound/SFX/SFX_CompendiumClose.SFX_CompendiumClose" 1.0 1.0 0.0 0 0))))

(event EventBeginPlay
  (bind _returnvalue (UserInterface|CreateWidget "/Game/Blueprint/CompendioSystemOLD/WBP_MainCompendio.WBP_MainCompendio_C" (Game|GetPlayerController 0)))
  (bind _output_get (Variables|Default|SetCompendio _returnvalue))
  (UserInterface|Viewport|AddtoViewport _output_get 0)
  (Widget|SetVisibility _output_get "Hidden")
  (Input|EnableInput (Game|GetPlayerController 0)))

(event Input|KeyboardEvents|C
  (params (Key :type Key%20Structure :default "None"))
  (bind _compendio (Variables|Default|GetCompendio))
  (bind _compendio_2 (Variables|Default|GetCompendio))
  (:Pressed
    (bind _output_get (Variables|Default|SetIs%20Compendium (not (Variables|Default|GetIs%20Compendium))))
    (if _output_get
      (Widget|SetVisibility _compendio "Visible")
      (Default|AddPage _compendio)
      (Default|AddPage _compendio 1)
      (Audio|PlaySound2D "/Game/Sound/SFX/SFX_CompendiumOpen.SFX_CompendiumOpen" 1.0 1.0 0.0 0 0)
      (else
        (Widget|SetVisibility _compendio_2 "Hidden")
        (Default|RemovePage _compendio_2)
        (Audio|PlaySound2D "/Game/Sound/SFX/SFX_CompendiumClose.SFX_CompendiumClose" 1.0 1.0 0.0 0 0)))))

(fn ConstructionScript)